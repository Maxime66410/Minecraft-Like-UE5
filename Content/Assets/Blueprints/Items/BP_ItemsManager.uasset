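; BP_ItemsManager is a world item pickup that spins in place and goes into the player's inventory on overlap.
; Shortly after BeginPlay it looks up its item by ID in a list, applies that item's mesh and per-slot or single shared material, then enables physics that ignores pawns.
; Tick keeps it upright while yawing it.
; Box overlap with BP_Player adds the item and, if accepted, plays a pop sound and destroys the actor.
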(event `self.ReceiveBeginPlay`
  (bind _list_items_list (break `/Game/Assets/Blueprints/Items/ST_Lists` (`self.List Items`)))
  (bind _staticmesh (`self.StaticMesh`))
  (`KismetSystemLibrary.Delay` 0.05)
  (set `self.CurrentItems` (`|GetArrayItem` _list_items_list (`self.CurrentItemsID`)))
  (`self.SetupModel`)
  (`self.SetupMaterials`)
  (`PrimitiveComponent.SetCollisionResponseToAllChannels` _staticmesh "ECR_Block")
  (`PrimitiveComponent.SetCollisionResponseToChannel` _staticmesh "ECC_Pawn" "ECR_Ignore")
  (`PrimitiveComponent.SetCollisionResponseToChannel` _staticmesh "ECC_WorldDynamic" "ECR_Overlap")
  (`PrimitiveComponent.SetSimulatePhysics` (`self.StaticMesh`) true))

(event `self.ReceiveTick`
  (params (DeltaSeconds :type "Float (single-precision)"))
  (`self.RotationAnim`))

(event `self.Box.OnComponentBeginOverlap`
  (params (OverlappedComponent :type "PrimitiveComponent Object Reference") (OtherActor :type "Actor Object Reference") (OtherComp :type "PrimitiveComponent Object Reference") (OtherBodyIndex :type Integer) (bFromSweep :type Boolean) (SweepResult :type "HitResult Structure (by ref)"))
  (bind _asbp_player (cast `/Game/Assets/Blueprints/Players/BP_Player` OtherActor))
  (bind _candestroyexit (`/Game/Assets/Blueprints/Players/BP_Player.AddItemInventory` _asbp_player (`self.CurrentItems`)))
  (if _candestroyexit
    (`GameplayStatics.PlaySoundAtLocation` "/Game/Assets/Audio/Player/pop.pop" (`self.K2_GetActorLocation`) (struct) 1.0 1.0 0.0 null null null null)
    (`self.K2_DestroyActor`)))

(fn `RotationAnim`
  (bind _staticmesh (`self.StaticMesh`))
  (bind (_returnvalue_roll _returnvalue_pitch _returnvalue_yaw) (`KismetMathLibrary.BreakRotator` (`SceneComponent.K2_GetComponentRotation` _staticmesh)))
  (`SceneComponent.K2_SetWorldRotation` _staticmesh (`KismetMathLibrary.MakeRotator` 0.0 0.0 (+ _returnvalue_yaw 1.0)) false false))

(fn `SetupMaterials`
  (bind _staticmesh (`self.StaticMesh`))
  (bind (_currentitems_id _currentitems_name _currentitems_staticmesh _currentitems_materials) (break `/Game/Assets/Blueprints/Items/ST_Items` (`self.CurrentItems`)))
  (for (_ _array_index) (`MeshComponent.GetMaterials` _staticmesh)
    (if (!= (`KismetArrayLibrary.Array_Length` _currentitems_materials) 1)
      (for (_array_element _array_index_2) _currentitems_materials
        (if (== _array_index_2 _array_index)
          (`PrimitiveComponent.SetMaterial` _staticmesh _array_index _array_element)))
      (else
        (`PrimitiveComponent.SetMaterial` _staticmesh _array_index (`|GetArrayItem` _currentitems_materials))))))

(fn `SetupModel`
  (bind (_currentitems_id _currentitems_name _currentitems_staticmesh) (break `/Game/Assets/Blueprints/Items/ST_Items` (`self.CurrentItems`)))
  (bind _staticmesh (`self.StaticMesh`))
  (`StaticMeshComponent.SetStaticMesh` _staticmesh _currentitems_staticmesh)
  (`SceneComponent.SetRelativeScale3D` _staticmesh (1.0 1.0 1.0)))

(fn `UserConstructionScript`)