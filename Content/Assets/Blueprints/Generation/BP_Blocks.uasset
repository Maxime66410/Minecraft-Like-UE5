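; Diggable voxel block actor for terrain generation, with Grass, Dirt, Stone and Sand types.
; SetupTexture assigns per-face materials and Resistance by BlockType, destroying Null and Air blocks.
; Dig decrements Resistance, playing random type-specific sounds; at zero it spawns a BP_ItemsManager drop carrying IDBlock and destroys itself.
; ResetDig restores the type's resistance, while SetStoneState converts the block to Stone and runs SetupTexture on a timer.
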(event `/Game/Assets/Blueprints/Generation/BPI_Blocks.Dig`
  (`/Engine/EditorBlueprintResources/StandardMacros.DecrementInt` (`self.Resistance`)
    (:`  `
      (if (== (`self.Resistance`) 0)
        (`self.DigSoundFinish`)
        (bind _returnvalue (`|SpawnActorFromClass` "/Game/Assets/Blueprints/Items/BP_ItemsManager.BP_ItemsManager_C" (`KismetMathLibrary.MakeTransform` (`self.K2_GetActorLocation`) (struct) (0.2 0.2 0.2)) "AdjustIfPossibleButAlwaysSpawn" "OverrideRootScale" null null))
        (set `/Game/Assets/Blueprints/Items/BP_ItemsManager.CurrentItemsID` (`self.IDBlock`) _returnvalue)
        (`self.K2_DestroyActor`)
        (else
          (`self.DigSound`))))))

(event `/Game/Assets/Blueprints/Generation/BPI_Blocks.ResetDig`
  (`self.ResetDigCount`))

(event `SetStoneState`
  (`KismetSystemLibrary.Delay` 0.2)
  (set `self.BlockType` "NewEnumerator4")
  (set `self.IDBlock` 3)
  (`KismetSystemLibrary.K2_SetTimer` null "SetupTexture" 1.0))

(fn `DigSound`
  (bind _returnvalue (select `int` (`KismetMathLibrary.RandomInteger` 5) :`0` "/Game/Assets/Audio/Dig/grass1.grass1" :`1` "/Game/Assets/Audio/Dig/grass2.grass2" :`2` "/Game/Assets/Audio/Dig/grass3.grass3" :`3` "/Game/Assets/Audio/Dig/grass4.grass4" :`4` "/Game/Assets/Audio/Dig/grass5.grass5" :`5` "/Game/Assets/Audio/Dig/grass6.grass6" :!type "SoundBase Object Reference"))
  (`GameplayStatics.PlaySoundAtLocation` (select `/Game/Assets/Blueprints/Generation/E_BlockType` (`self.BlockType`) :`NewEnumerator2` _returnvalue :`NewEnumerator3` _returnvalue :`NewEnumerator4` (select `int` (`KismetMathLibrary.RandomInteger` 5) :`0` "/Game/Assets/Audio/Dig/stone1.stone1" :`1` "/Game/Assets/Audio/Dig/stone2.stone2" :`2` "/Game/Assets/Audio/Dig/stone3.stone3" :`3` "/Game/Assets/Audio/Dig/stone4.stone4" :`4` "/Game/Assets/Audio/Dig/stone5.stone5" :`5` "/Game/Assets/Audio/Dig/stone6.stone6" :!type "SoundBase Object Reference") :`NewEnumerator7` (select `int` (`KismetMathLibrary.RandomInteger` 4) :`0` "/Game/Assets/Audio/Dig/sand1.sand1" :`1` "/Game/Assets/Audio/Dig/sand2.sand2" :`2` "/Game/Assets/Audio/Dig/sand3.sand3" :`3` "/Game/Assets/Audio/Dig/sand4.sand4" :`4` "/Game/Assets/Audio/Dig/sand5.sand5" :!type "SoundBase Object Reference")) (`self.K2_GetActorLocation`) (struct) 1.0 0.6 0.0 null null null null))

(fn `DigSoundFinish`
  (bind _returnvalue (select `int` (`KismetMathLibrary.RandomInteger` 3) :`0` "/Game/Assets/Audio/Dig/Finish/grass1.grass1" :`1` "/Game/Assets/Audio/Dig/Finish/grass2.grass2" :`2` "/Game/Assets/Audio/Dig/Finish/grass3.grass3" :`3` "/Game/Assets/Audio/Dig/Finish/grass4.grass4" :!type "SoundBase Object Reference"))
  (`GameplayStatics.PlaySoundAtLocation` (select `/Game/Assets/Blueprints/Generation/E_BlockType` (`self.BlockType`) :`NewEnumerator2` _returnvalue :`NewEnumerator3` _returnvalue :`NewEnumerator4` (select `int` (`KismetMathLibrary.RandomInteger` 3) :`0` "/Game/Assets/Audio/Dig/Finish/stone1.stone1" :`1` "/Game/Assets/Audio/Dig/Finish/stone2.stone2" :`2` "/Game/Assets/Audio/Dig/Finish/stone3.stone3" :`3` "/Game/Assets/Audio/Dig/Finish/stone4.stone4" :!type "SoundBase Object Reference") :`NewEnumerator7` (select `int` (`KismetMathLibrary.RandomInteger` 3) :`0` "/Game/Assets/Audio/Dig/Finish/sand1.sand1" :`1` "/Game/Assets/Audio/Dig/Finish/sand2.sand2" :`2` "/Game/Assets/Audio/Dig/Finish/sand3.sand3" :`3` "/Game/Assets/Audio/Dig/Finish/sand4.sand4" :!type "SoundBase Object Reference")) (`self.K2_GetActorLocation`) (struct) 1.0 1.0 0.0 null null null null))

(fn `ResetDigCount`
  (switch `/Game/Assets/Blueprints/Generation/E_BlockType` (`self.BlockType`)
    (:`NewEnumerator0`
      ;[1 1 1] NULL
      (set `self.Resistance` 0 :!label _label))
    (:`NewEnumerator1`
      (goto _label))
    (:`NewEnumerator2`
      ;[1 1 1] LOW
      (set `self.Resistance` 3 :!label _label_2))
    (:`NewEnumerator3`
      (goto _label_2))
    (:`NewEnumerator4`
      ;[1 1 1] MEDIUM
      (set `self.Resistance` 6))
    (:`NewEnumerator7`
      (goto _label_2))))

(fn `SetupTexture`
  (bind _staticmesh (`self.StaticMesh`))
  (bind _staticmesh_2 (`self.StaticMesh`))
  (bind _staticmesh_3 (`self.StaticMesh`))
  (bind _staticmesh_4 (`self.StaticMesh`))
  (switch `/Game/Assets/Blueprints/Generation/E_BlockType` (`self.BlockType`)
    (:`NewEnumerator0`
      (`self.K2_DestroyActor`))
    (:`NewEnumerator1`
      (`self.K2_DestroyActor`))
    (:`NewEnumerator2`
      ;[1 1 1] Grass Block
      (`PrimitiveComponent.SetMaterial` _staticmesh_3 0 "/Game/Assets/Texture/Blocks/M_BlockGrassMaster_BasicGrassSide.M_BlockGrassMaster_BasicGrassSide")
      (`PrimitiveComponent.SetMaterial` _staticmesh_3 1 "/Game/Assets/Texture/Blocks/M_BlockGrassMaster_BasicGrassTop.M_BlockGrassMaster_BasicGrassTop")
      (`PrimitiveComponent.SetMaterial` _staticmesh_3 2 "/Game/Assets/Texture/Blocks/M_BlockGrassMaster_BasicGrassSide.M_BlockGrassMaster_BasicGrassSide")
      (`PrimitiveComponent.SetMaterial` _staticmesh_3 3 "/Game/Assets/Texture/Blocks/M_BlockMasters_Dirt.M_BlockMasters_Dirt")
      (`PrimitiveComponent.SetMaterial` _staticmesh_3 4 "/Game/Assets/Texture/Blocks/M_BlockGrassMaster_BasicGrassSide.M_BlockGrassMaster_BasicGrassSide")
      (`PrimitiveComponent.SetMaterial` _staticmesh_3 5 "/Game/Assets/Texture/Blocks/M_BlockGrassMaster_BasicGrassSide.M_BlockGrassMaster_BasicGrassSide")
      (set `self.Resistance` 3))
    (:`NewEnumerator3`
      ;[1 1 1] Dirt
      (`PrimitiveComponent.SetMaterial` _staticmesh 0 "/Game/Assets/Texture/Blocks/M_BlockMasters_Dirt.M_BlockMasters_Dirt")
      (`PrimitiveComponent.SetMaterial` _staticmesh 1 "/Game/Assets/Texture/Blocks/M_BlockMasters_Dirt.M_BlockMasters_Dirt")
      (`PrimitiveComponent.SetMaterial` _staticmesh 2 "/Game/Assets/Texture/Blocks/M_BlockMasters_Dirt.M_BlockMasters_Dirt")
      (`PrimitiveComponent.SetMaterial` _staticmesh 3 "/Game/Assets/Texture/Blocks/M_BlockMasters_Dirt.M_BlockMasters_Dirt")
      (`PrimitiveComponent.SetMaterial` _staticmesh 4 "/Game/Assets/Texture/Blocks/M_BlockMasters_Dirt.M_BlockMasters_Dirt")
      (`PrimitiveComponent.SetMaterial` _staticmesh 5 "/Game/Assets/Texture/Blocks/M_BlockMasters_Dirt.M_BlockMasters_Dirt")
      (set `self.Resistance` 3))
    (:`NewEnumerator4`
      ;[1 1 1] Stone
      (`PrimitiveComponent.SetMaterial` _staticmesh_4 0 "/Game/Assets/Texture/Blocks/M_BlockMasters_Stone.M_BlockMasters_Stone")
      (`PrimitiveComponent.SetMaterial` _staticmesh_4 1 "/Game/Assets/Texture/Blocks/M_BlockMasters_Stone.M_BlockMasters_Stone")
      (`PrimitiveComponent.SetMaterial` _staticmesh_4 2 "/Game/Assets/Texture/Blocks/M_BlockMasters_Stone.M_BlockMasters_Stone")
      (`PrimitiveComponent.SetMaterial` _staticmesh_4 3 "/Game/Assets/Texture/Blocks/M_BlockMasters_Stone.M_BlockMasters_Stone")
      (`PrimitiveComponent.SetMaterial` _staticmesh_4 4 "/Game/Assets/Texture/Blocks/M_BlockMasters_Stone.M_BlockMasters_Stone")
      (`PrimitiveComponent.SetMaterial` _staticmesh_4 5 "/Game/Assets/Texture/Blocks/M_BlockMasters_Stone.M_BlockMasters_Stone")
      (set `self.Resistance` 6))
    (:`NewEnumerator7`
      ;[1 1 1] Sand
      (`PrimitiveComponent.SetMaterial` _staticmesh_2 0 "/Game/Assets/Texture/Blocks/M_BlockMasters_Sand.M_BlockMasters_Sand")
      (`PrimitiveComponent.SetMaterial` _staticmesh_2 1 "/Game/Assets/Texture/Blocks/M_BlockMasters_Sand.M_BlockMasters_Sand")
      (`PrimitiveComponent.SetMaterial` _staticmesh_2 2 "/Game/Assets/Texture/Blocks/M_BlockMasters_Sand.M_BlockMasters_Sand")
      (`PrimitiveComponent.SetMaterial` _staticmesh_2 3 "/Game/Assets/Texture/Blocks/M_BlockMasters_Sand.M_BlockMasters_Sand")
      (`PrimitiveComponent.SetMaterial` _staticmesh_2 4 "/Game/Assets/Texture/Blocks/M_BlockMasters_Sand.M_BlockMasters_Sand")
      (`PrimitiveComponent.SetMaterial` _staticmesh_2 5 "/Game/Assets/Texture/Blocks/M_BlockMasters_Sand.M_BlockMasters_Sand")
      (set `self.Resistance` 3))))

(fn `UserConstructionScript`)