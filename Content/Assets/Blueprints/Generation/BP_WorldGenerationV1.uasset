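; Generates a blocky voxel terrain of BP_Blocks actors on a Width by Length grid.
; The construction script previews the surface with instanced meshes, using three summed layers of sine-product height, rounded to block steps.
; On BeginPlay, GenerateWorld destroys that preview and spawns an actor per surface cell plus ten beneath it.
; Block types follow height and depth: surface at or below zero differs from higher ground, with upper subsurface and deep layers below.
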(event `self.ReceiveBeginPlay`
  (`self.GenerateWorld`))

(fn `GenerateWorld`
  (locals (OldBlock :type "/Game/Assets/Blueprints/Generation/BP_Blocks Object Reference"))
  (bind _f1 (`self.F1`))
  (bind _f2 (`self.F2`))
  (bind _f3 (`self.F3`))
  (`ActorComponent.K2_DestroyComponent` (`self.InstancedStaticMesh`))
  (for _index (range (+ (`self.Width`) 1))
    (for _index_2 (range (+ (`self.Length`) 1))
      (bind _returnvalue (`KismetMathLibrary.MakeVector` (`KismetMathLibrary.Conv_IntToDouble` (* _index (`self.Xoffset`))) (`KismetMathLibrary.Conv_IntToDouble` (* _index_2 (`self.Yoffset`))) (* (`KismetMathLibrary.Conv_IntToDouble` (`KismetMathLibrary.Round` (+ (* (`KismetMathLibrary.DegSin` (* _index _f1)) (`KismetMathLibrary.DegSin` (* _index_2 _f1)) (`self.H1`)) (* (`KismetMathLibrary.DegSin` (* _index _f2)) (`KismetMathLibrary.DegSin` (* _index_2 _f2)) (`self.H2`)) (* (`KismetMathLibrary.DegSin` (* _index _f3)) (`KismetMathLibrary.DegSin` (* _index_2 _f3)) (`self.H3`))))) 100.0)))
      (bind _returnvalue_2 (`|SpawnActorFromClass` "/Game/Assets/Blueprints/Generation/BP_Blocks.BP_Blocks_C" (`KismetMathLibrary.MakeTransform` _returnvalue) "Undefined" "OverrideRootScale" null null))
      (set `local.OldBlock` _returnvalue_2)
      (if (<= (.z _returnvalue) 0.0)
        (set `/Game/Assets/Blueprints/Generation/BP_Blocks.BlockType` "NewEnumerator7" _returnvalue_2)
        (else
          (set `/Game/Assets/Blueprints/Generation/BP_Blocks.BlockType` "NewEnumerator2" _returnvalue_2)))
      ;[1 1 1] Hauteur
      (for _index_3 (range 1 11)
        (bind _returnvalue_3 (`|SpawnActorFromClass` "/Game/Assets/Blueprints/Generation/BP_Blocks.BP_Blocks_C" (`KismetMathLibrary.MakeTransform` (`KismetMathLibrary.MakeVector` (.x _returnvalue) (.y _returnvalue) (+ (.z _returnvalue) (* _index_3 -100)))) "Undefined" "OverrideRootScale" null null))
        (if (< _index_3 3)
          (if (`|EnumEquality` (`/Game/Assets/Blueprints/Generation/BP_Blocks.BlockType` (`local.OldBlock`)) "NewEnumerator7")
            (set `/Game/Assets/Blueprints/Generation/BP_Blocks.BlockType` "NewEnumerator7" _returnvalue_3)
            (else
              (set `/Game/Assets/Blueprints/Generation/BP_Blocks.BlockType` "NewEnumerator3" _returnvalue_3)))
          (else
            (set `/Game/Assets/Blueprints/Generation/BP_Blocks.BlockType` "NewEnumerator4" _returnvalue_3)))))))

(fn `UserConstructionScript`
  (bind _f1 (`self.F1`))
  (bind _f2 (`self.F2`))
  (bind _f3 (`self.F3`))
  ;[1 1 1] SIMPLE PREVIEW
  (for _index (range (+ (`self.Width`) 1))
    (for _index_2 (range (+ (`self.Length`) 1))
      (`InstancedStaticMeshComponent.AddInstance` (`self.InstancedStaticMesh`) (`KismetMathLibrary.MakeTransform` (`KismetMathLibrary.MakeVector` (`KismetMathLibrary.Conv_IntToDouble` (* _index (`self.Xoffset`))) (`KismetMathLibrary.Conv_IntToDouble` (* _index_2 (`self.Yoffset`))) (* (`KismetMathLibrary.Conv_IntToDouble` (`KismetMathLibrary.Round` (+ (* (`KismetMathLibrary.DegSin` (* _index _f1)) (`KismetMathLibrary.DegSin` (* _index_2 _f1)) (`self.H1`)) (* (`KismetMathLibrary.DegSin` (* _index _f2)) (`KismetMathLibrary.DegSin` (* _index_2 _f2)) (`self.H2`)) (* (`KismetMathLibrary.DegSin` (* _index _f3)) (`KismetMathLibrary.DegSin` (* _index_2 _f3)) (`self.H3`))))) 100.0))) false))))