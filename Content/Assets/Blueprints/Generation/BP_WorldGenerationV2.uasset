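; World generator actor that builds stepped block terrain from a grid of instanced static meshes sized by Width and Length.
; Height sums three sine-product layers with separate frequencies and amplitudes, rounded into 100-unit steps to form plateaus.
; The construction script previews the terrain, and GenerateWorld repeats the same loop on BeginPlay without clearing instances.
; ChangeMaterials is an uncalled stub that only tests a transform's height.
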(event `self.ReceiveBeginPlay`
  (`self.GenerateWorld`))

(fn `ChangeMaterials`
  (params (TR :type "Transform Structure"))
  (locals (TRLocal :type "Transform Structure"))
  (bind _output_get (set `local.TRLocal` TR))
  (if (> (.z (.location _output_get)) 10000.0)
    _))

(fn `GenerateWorld`
  (locals (OldBlock :type "/Game/Assets/Blueprints/Generation/BP_Blocks Object Reference"))
  (bind _f1 (`self.F1`))
  (bind _f2 (`self.F2`))
  (bind _f3 (`self.F3`))
  (for _index (range (+ (`self.Width`) 1))
    (for _index_2 (range (+ (`self.Length`) 1))
      (`InstancedStaticMeshComponent.AddInstance` (`self.InstancedStaticMesh`) (`KismetMathLibrary.MakeTransform` (`KismetMathLibrary.MakeVector` (`KismetMathLibrary.Conv_IntToDouble` (* _index (`self.Xoffset`))) (`KismetMathLibrary.Conv_IntToDouble` (* _index_2 (`self.Yoffset`))) (* (`KismetMathLibrary.Conv_IntToDouble` (`KismetMathLibrary.Round` (+ (* (`KismetMathLibrary.DegSin` (* _index _f1)) (`KismetMathLibrary.DegSin` (* _index_2 _f1)) (`self.H1`)) (* (`KismetMathLibrary.DegSin` (* _index _f2)) (`KismetMathLibrary.DegSin` (* _index_2 _f2)) (`self.H2`)) (* (`KismetMathLibrary.DegSin` (* _index _f3)) (`KismetMathLibrary.DegSin` (* _index_2 _f3)) (`self.H3`))))) 100.0))) false))))

(fn `UserConstructionScript`
  (bind _f1 (`self.F1`))
  (bind _f2 (`self.F2`))
  (bind _f3 (`self.F3`))
  ;[1 1 1] SIMPLE PREVIEW
  (for _index (range (+ (`self.Width`) 1))
    (for _index_2 (range (+ (`self.Length`) 1))
      (`InstancedStaticMeshComponent.AddInstance` (`self.InstancedStaticMesh`) (`KismetMathLibrary.MakeTransform` (`KismetMathLibrary.MakeVector` (`KismetMathLibrary.Conv_IntToDouble` (* _index (`self.Xoffset`))) (`KismetMathLibrary.Conv_IntToDouble` (* _index_2 (`self.Yoffset`))) (* (`KismetMathLibrary.Conv_IntToDouble` (`KismetMathLibrary.Round` (+ (* (`KismetMathLibrary.DegSin` (* _index _f1)) (`KismetMathLibrary.DegSin` (* _index_2 _f1)) (`self.H1`)) (* (`KismetMathLibrary.DegSin` (* _index _f2)) (`KismetMathLibrary.DegSin` (* _index_2 _f2)) (`self.H2`)) (* (`KismetMathLibrary.DegSin` (* _index _f3)) (`KismetMathLibrary.DegSin` (* _index_2 _f3)) (`self.H3`))))) 100.0))) false))))